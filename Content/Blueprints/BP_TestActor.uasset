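; Test actor that visualizes Azure Kinect body tracking by driving one component per skeleton joint.
; BeginPlay initializes and logs device 0, and EndPlay shuts it down.
; The construction script fills VisualJoints in Kinect joint index order, from pelvis to right ear.
; Tick acquires the first tracked body if none is valid, sets it mirrored, and copies each joint's position and orientation to the matching component's relative transform.
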(event `self.ReceiveBeginPlay`
  (bind _returnvalue (`AzureKinectManager.GetBodies` 0))
  (`AzureKinectManager.InitDevice` 0 "NFOV_UNBINNED" 33)
  (`KismetSystemLibrary.PrintString` "Initializing Azure Kinect" true true (struct :`G` 0.66 :`B` 1.0 :`A` 1.0) 10.0)
  (`AzureKinectManager.ToggleDeviceLogging` 0 true true)
  (if (> (`KismetArrayLibrary.Array_Length` _returnvalue) 0)
    (bind _output_get (set `self.KinectBody` (`|GetArrayItem` _returnvalue)))
    (set `AzureKinectBody.bIsMirrored` true _output_get)))

(event `self.ReceiveTick`
  (params (DeltaSeconds :type "Float (single-precision)"))
  (bind _returnvalue (`AzureKinectManager.GetBodies` 0))
  (`self.KinectBody`
    (:`then`
      (set `self.KinectJoints` (`AzureKinectBody.GetJoints` (`self.KinectBody`)) :!label _label)
      (for (_array_element _array_index) (`self.VisualJoints`)
        (bind (_position _orientation) (break `AzureKinectJoint` (`|GetArrayItem` (`self.KinectJoints`) _array_index)))
        (`SceneComponent.K2_SetRelativeLocationAndRotation` _array_element _position _orientation false false)))
    (:`else`
      (if (> (`KismetArrayLibrary.Array_Length` _returnvalue) 0)
        (bind _output_get (set `self.KinectBody` (`|GetArrayItem` _returnvalue)))
        (`/Engine/EditorBlueprintResources/StandardMacros.IsValid` _output_get
          (:`Is Valid`
            (set `AzureKinectBody.bIsMirrored` true _output_get)
            (goto _label)))))))

(event `self.ReceiveEndPlay`
  (params (EndPlayReason :type "EEndPlayReason Enum" :default "Destroyed"))
  (`AzureKinectManager.ShutdownDevice` 0))

(fn `UserConstructionScript`
  (set `self.VisualJoints` (`|MakeArray` (`self.0_Pelvis`) (`self.1_SpineNaval`) (`self.2_SpineChest`) (`self.3_Neck`) (`self.4_ClavicleLeft`) (`self.5_ShoulderLeft`) (`self.6_ElbowLeft`) (`self.7_WristLeft`) (`self.8_HandLeft`) (`self.9_HandTipLeft`) (`self.10_ThumbLeft`) (`self.11_ClavicleRight`) (`self.12_ShoulderRight`) (`self.13_ElbowRight`) (`self.14_WristRight`) (`self.15_HandRight`) (`self.16_HandTipRight`) (`self.17_ThumbRight`) (`self.18_HipLeft`) (`self.19_KneeLeft`) (`self.20_AnkleLeft`) (`self.21_FootLeft`) (`self.22_HipRight`) (`self.23_KneeRight`) (`self.24_AnkleRight`) (`self.25_FootRight`) (`self.26_Head`) (`self.27_Nose`) (`self.28_EyeLeft`) (`self.29_EarLeft`) (`self.30_EyeRight`) (`self.31_EarRight`) :!type "SceneComponent Object Reference")))