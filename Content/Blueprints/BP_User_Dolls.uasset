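; Actor that drives user doll avatars from two Azure Kinect body-tracking devices.
; BeginPlay initializes both devices and caches hidden meshes with their BP_AnimUserDoll instances.
; Tick updates only the first doll's visibility and joint transforms, plus the tracked count, using device 0.
; Low-confidence joints borrow device 1's rotation, yaw-corrected by AzureAngleBetween, while SetSkeletalMesh picks a kid, male or female doll from user height and sex.
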(event `self.ReceiveBeginPlay`
  (`AzureKinectManager.InitDevice` 0 "WFOV_2X2BINNED" 33)
  (`AzureKinectManager.InitDevice` 1 "WFOV_2X2BINNED" 33)
  (`AzureKinectManager.ToggleDeviceLogging` 0 true true)
  (`KismetSystemLibrary.PrintString` "Initializing Azure Kinect" false false (struct :`G` 0.66 :`B` 1.0 :`A` 1.0) 10.0)
  (bind _asmain_game_instance (cast `MainGameInstance` (`GameplayStatics.GetGameInstance`)))
  (set `self.Main Game Instance` _asmain_game_instance)
  (set `self.Azure Angle Between` (`MainGameInstance.Azure_angle_between` _asmain_game_instance))
  (`self.MakeSkeletalMeshArray`)
  (for _array_element (`self.SkeletalMeshes`)
    (`SceneComponent.K2_SetRelativeTransform` _array_element (`self.DefaultTransform`) false true)
    (`SceneComponent.SetVisibility` _array_element false false)
    (bind _asbp_anim_user_doll (cast `/Game/Blueprints/BP_AnimUserDoll` (`SkeletalMeshComponent.GetAnimInstance` _array_element)))
    (set `/Game/Blueprints/BP_AnimUserDoll.TransformAlpha` 1.0 _asbp_anim_user_doll)
    (`KismetArrayLibrary.Array_Add` (`self.AnimBPs`) _asbp_anim_user_doll))
  (set `self.KinectBodies0` (`AzureKinectManager.GetBodies` 0))
  (set `self.KinectBodies1` (`AzureKinectManager.GetBodies` 1)))

(event `self.ReceiveTick`
  (params (DeltaSeconds :type "Float (single-precision)"))
  (bind _skeletalmeshes (`self.SkeletalMeshes`))
  (bind _main_game_instance (`self.Main Game Instance`))
  (bind _kinectbodies1 (`self.KinectBodies1`))
  (set `MainGameInstance.TrackedSkeleton_Num` 0 (`self.Main Game Instance`))
  (if (`AzureKinectManager.IsDeviceInitialized` 0)
    (for (_array_element _array_index) (`self.KinectBodies0`)
      (`/Engine/EditorBlueprintResources/StandardMacros.IsValid` _array_element
        (:`Is Valid`
          (bind _output (`|GetArrayItem` _skeletalmeshes _array_index))
          (if (== _output (`|GetArrayItem` _skeletalmeshes))
            (bind _bistracked (`AzureKinectBody.bIsTracked` _array_element))
            (`SceneComponent.SetVisibility` _output _bistracked false)
            (if _bistracked
              (set `MainGameInstance.TrackedSkeleton_Num` (+ (`MainGameInstance.TrackedSkeleton_Num` _main_game_instance) 1) _main_game_instance)
              (for (_array_element_2 _array_index_2) (`AzureKinectBody.GetJoints` _array_element)
                (bind (_position _orientation _confidence _positionmultiplier _index _customindex) (break `AzureKinectJoint` _array_element_2))
                ;[1 1 1] 코멘트
                (if (`|EnumEquality` _customindex (`self.NewVar_0`))
                  (`KismetSystemLibrary.PrintString` (`KismetStringLibrary.Conv_RotatorToString` _orientation) false false (struct :`G` 0.66 :`B` 1.0 :`A` 1.0) 200.0))
                (if (>= _confidence 1)
                  (bind _jointstransform (`/Game/Blueprints/BP_AnimUserDoll.JointsTransform` (`|GetArrayItem` (`self.AnimBPs`) _array_index)))
                  (`KismetArrayLibrary.Array_Set` _jointstransform _array_index_2 (`KismetMathLibrary.MakeTransform` _position _orientation) :!label _label)
                  (else
                    (`KismetSystemLibrary.PrintString` (`KismetStringLibrary.Conv_IntToString` _index) false false (struct :`G` 0.66 :`B` 1.0 :`A` 1.0) 1.0)
                    (if (`KismetArrayLibrary.Array_IsValidIndex` _kinectbodies1)
                      (bind (_position_2 _orientation_2 _confidence_2) (break `AzureKinectJoint` (`AzureKinectBody.GetJoint` (`|GetArrayItem` _kinectbodies1 _array_index) _array_index_2)))
                      (if (>= _confidence_2 1)
                        (`KismetArrayLibrary.Array_Set` _jointstransform _array_index_2 (`KismetMathLibrary.MakeTransform` _position (`KismetMathLibrary.MakeRotator` (.roll _orientation_2) (.pitch _orientation_2) (- (.yaw _orientation_2) (`self.Azure Angle Between`)))))
                        (else
                          (goto _label)))
                      (else
                        (goto _label)))))))))
        (:`Is Not Valid`
          (`SceneComponent.SetVisibility` _output false false))))))

(event `self.ReceiveEndPlay`
  (params (EndPlayReason :type "EEndPlayReason Enum" :default "Destroyed"))
  (`AzureKinectManager.ShutdownDevice` 0)
  (`AzureKinectManager.ShutdownDevice` 1))

(fn `MakeSkeletalMeshArray`
  (set `self.SkeletalMeshes` (`|MakeArray` (`self.SkeletalMesh0`) (`self.SkeletalMesh1`) (`self.SkeletalMesh2`) (`self.SkeletalMesh3`) (`self.SkeletalMesh4`) (`self.SkeletalMesh5`) (`self.SkeletalMesh6`) (`self.SkeletalMesh7`) (`self.SkeletalMesh8`) (`self.SkeletalMesh9`)))
  (return))

(fn `SetSkeletalMesh`
  (bind _skeletalmesh0 (`self.SkeletalMesh0`))
  (bind _skeletalmesh0_2 (`self.SkeletalMesh0`))
  (bind _skeletalmesh0_3 (`self.SkeletalMesh0`))
  (bind _asmain_game_instance (cast `MainGameInstance` (`GameplayStatics.GetGameInstance`)))
  (if (<= (`MainGameInstance.User_Hight` _asmain_game_instance) 140)
    (`SkinnedMeshComponent.SetSkinnedAssetAndUpdate` _skeletalmesh0_2 "/Game/Character/User_Doll/SK_HS_kidDoll_ueJoint.SK_HS_kidDoll_ueJoint" true)
    (`SceneComponent.SetRelativeScale3D` _skeletalmesh0_2 (0.8 0.8 0.8))
    (elif (`KismetStringLibrary.EqualEqual_StrStr` (`MainGameInstance.User_Sex` _asmain_game_instance) "남자")
      (`SkinnedMeshComponent.SetSkinnedAssetAndUpdate` _skeletalmesh0_3 "/Game/Character/User_Doll/SK_HS_maleDoll_ueJoint.SK_HS_maleDoll_ueJoint" true)
      (`SceneComponent.SetRelativeScale3D` _skeletalmesh0_3 (1.0 1.0 1.0))
      (else
        (`SkinnedMeshComponent.SetSkinnedAssetAndUpdate` _skeletalmesh0 "/Game/Character/User_Doll/SK_HS_femaleDoll_ueJoint.SK_HS_femaleDoll_ueJoint" true)
        (`SceneComponent.SetRelativeScale3D` _skeletalmesh0 (1.0 1.0 1.0))))))

(fn `UserConstructionScript`)